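; BP_HealthSpawnPoint is a spawn point that creates BP_HealthPickUp actors at its Scene component's world transform.
; While HasPickUP is false, Tick accumulates delta time in Timer and spawns a pickup once it exceeds Cooldown, ignoring collisions.
; The timer resets after each spawn, but nothing in this Blueprint sets HasPickUP, so spawning repeats unless that flag changes elsewhere.
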(event `self.ReceiveTick`
  (params (DeltaSeconds :type "Float (single-precision)"))
  (if (not (`self.HasPickUP`))
    (bind _output_get (set `self.Timer` (+ (`self.Timer`) DeltaSeconds)))
    (if (> _output_get (`self.Cooldown`))
      (`|SpawnActorFromClass` "/Game/Blueprints/BP_HealthPickUp.BP_HealthPickUp_C" (`SceneComponent.K2_GetComponentToWorld` (`self.Scene`)) "AlwaysSpawn" "MultiplyWithRoot" null null)
      (set `self.Timer` 0.0))))

(fn `UserConstructionScript`)