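; BP_GameOverPortalSpawner is a placed actor that spawns the game-over portal at its own transform when no enemies remain.
; Each Tick it casts the game mode to GM_Drone and polls the EnemyManager's current enemy count.
; At zero or below it sets Spawned and calls GameOver, which spawns BP_GameOverPortal.
; The Spawned check has empty branches, so as written it does not prevent repeat spawns on later ticks.
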(event `self.ReceiveBeginPlay`)

(event `self.ReceiveTick`
  (params (DeltaSeconds :type "Float (single-precision)"))
  (bind _asgm_drone (cast `/Game/Core/GM_Drone` (`GameplayStatics.GetGameMode`)))
  (if (<= (`/Game/Blueprints/Enemies/EnemyManager.CurrentEnemyNumber` (`/Game/Core/GM_Drone.EnemyManager` _asgm_drone)) 0)
    (if (`self.Spawned`)
      _
      (else
        _))
    (set `self.Spawned` true)
    (`self.GameOver`)))

(fn `GameOver`
  (`|SpawnActorFromClass` "/Game/Blueprints/Portal/BP_GameOverPortal.BP_GameOverPortal_C" (`self.GetTransform`) "Undefined" "MultiplyWithRoot" null null))

(fn `UserConstructionScript`)