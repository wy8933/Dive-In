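; Behavior tree task that moves a BP_EnemyBase pawn toward its blackboard target using AIMoveTo.
; It projects the TargetActor's location onto the navmesh with a narrow, very tall extent, falling back to TargetPosition if the actor is invalid or projection fails.
; HasArrived is cleared when the move starts and set on success, which finishes the task.
; A failed move has no handler, so it never calls FinishExecute.
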(event `self.ReceiveExecuteAI`
  (params (OwnerController :type "AIController Object Reference") (ControlledPawn :type "Pawn Object Reference"))
  (bind _returnvalue (`AIBlueprintHelperLibrary.GetBlackboard` OwnerController))
  (bind _returnvalue_2 (`BlackboardComponent.GetValueAsObject` _returnvalue "TargetActor"))
  (bind _asbp_enemy_base (cast `/Game/Blueprints/Enemies/BP_EnemyBase` ControlledPawn))
  (`/Engine/EditorBlueprintResources/StandardMacros.IsValid` _returnvalue_2
    (:`Is Valid`
      (bind _asactor (cast `Actor` _returnvalue_2))
      (bind (_projectedlocation _returnvalue_3) (`NavigationSystemV1.K2_ProjectPointToNavigation` (`Actor.K2_GetActorLocation` _asactor) null null (`KismetMathLibrary.MakeVector` 1.0 1.0 10000.0)))
      (if _returnvalue_3
        (`|AIMoveTo` _asbp_enemy_base _projectedlocation null
          (:`then`
            (`BlackboardComponent.SetValueAsBool` _returnvalue "HasArrived" false :!label _label))
          (:`OnSuccess`
            (`/Engine/EditorBlueprintResources/StandardMacros.IsValid` _returnvalue :!label _label_2
              (:`Is Valid`
                (`BlackboardComponent.SetValueAsBool` _returnvalue "HasArrived" true)
                (`self.FinishExecute` true)))))
        (else
          (`|AIMoveTo` _asbp_enemy_base (`BlackboardComponent.GetValueAsVector` _returnvalue "TargetPosition") null :!label _label_3
            (:`then`
              (goto _label))
            (:`OnSuccess`
              (goto _label_2))))))
    (:`Is Not Valid`
      (goto _label_3))))