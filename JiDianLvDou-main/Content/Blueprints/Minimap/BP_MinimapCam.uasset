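; BP_MinimapCam is a scene capture actor that follows the player's drone to feed a minimap.
; On BeginPlay it creates and shows WBP_MinimapUI targeting the player pawn, then caches the BP_Drone and hides it from its SceneCaptureComponent2D.
; Each Tick it moves itself to the drone's RotationCenter world location without sweeping.
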(event `self.ReceiveBeginPlay`
  (bind _returnvalue (`|CreateWidget` "/Game/Blueprints/WBP/WBP_MinimapUI.WBP_MinimapUI_C" (`GameplayStatics.GetPlayerController` 0)))
  (set `/Game/Blueprints/WBP/WBP_MinimapUI.Target` (`GameplayStatics.GetPlayerPawn` 0) _returnvalue)
  (`UserWidget.AddToViewport` _returnvalue 0)
  (`Widget.SetVisibility` _returnvalue "Visible")
  (bind _asbp_drone (cast `/Game/Blueprints/Drone/BP_Drone` (`GameplayStatics.GetPlayerPawn` 0)))
  (set `self.Drone` _asbp_drone)
  (set `SceneCaptureComponent.HiddenActors` (`|MakeArray` (`self.Drone`) :!type "Actor Object Reference") (`self.SceneCaptureComponent2D`)))

(event `self.ReceiveTick`
  (params (DeltaSeconds :type "Float (single-precision)"))
  (`self.K2_SetActorLocation` self (`SceneComponent.K2_GetComponentLocation` (`/Game/Blueprints/Drone/BP_Drone.RotationCenter` (`self.Drone`))) false true))

(fn `UserConstructionScript`)