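; Base zombie enemy for the drone player, killed by damage or by body-part inflation.
; Pawn sensing, sight-loss timeout and hits update AI blackboard keys for patrol, chase and attack.
; Inflation slows it; one full part stops its AI and floats it into a portal spawned overhead.
; Either death adds score, spawns an EXP orb, reports to the enemy manager and destroys the actor.
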(event `self.ReceiveBeginPlay`)

(event `self.ReceiveTick`
  (params (DeltaSeconds :type "Float (single-precision)"))
  (if (`self.IsFloating`)
    (`self.K2_AddActorWorldOffset` (`KismetMathLibrary.MakeVector` 0.0 0.0 (* DeltaSeconds (`self.FloatingSpeed`))) true)
    (if (< (`KismetMathLibrary.Vector_Distance` (`self.K2_GetActorLocation`) (`self.FloatingTarget`)) 100.0)
      (`/Game/Blueprints/Portal/BP_Portal.EnemyEntered` (`self.Portal`))
      (`self.Die` true))
    (else
      (set `self.AttackTimer` (- (`self.AttackTimer`) DeltaSeconds))
      (if (> (- (`KismetSystemLibrary.GetGameTimeInSeconds`) (`self.LastTimeSawPlayer`)) (`self.DelayBeforeLoseSight`))
        (`BlackboardComponent.SetValueAsBool` (`self.BB`) "IsInAttackRange" false)
        (if (not (`self.AlwaysChasePlayer`))
          (`BlackboardComponent.ClearValue` (`self.BB`) "TargetActor")
          (if (`BlackboardComponent.GetValueAsBool` (`self.BB`) "HasArrived")
            (if (`BlackboardComponent.GetValueAsBool` (`self.BB`) "IsChasing")
              (`BlackboardComponent.SetValueAsBool` (`self.BB`) "HasTarget" false)
              (else
                (`self.K2_DestroyActor`)))))))))

(event `self.PawnSensing.OnSeePawn`
  (params (Pawn :type "Pawn Object Reference"))
  (bind _returnvalue (`self.K2_GetActorLocation` Pawn))
  (bind (_projectedlocation _returnvalue_2) (`NavigationSystemV1.K2_ProjectPointToNavigation` _returnvalue null null (`KismetMathLibrary.MakeVector` 1.0 1.0 10000.0)))
  (if (`self.ActorHasTag` Pawn "Player")
    (if _returnvalue_2
      (`BlackboardComponent.SetValueAsVector` (`self.BB`) "TargetPosition" _projectedlocation))
    (`BlackboardComponent.SetValueAsObject` (`self.BB`) "TargetActor" Pawn)
    (`BlackboardComponent.SetValueAsBool` (`self.BB`) "IsInAttackRange" (< (`KismetMathLibrary.Vector_Distance` (`self.K2_GetActorLocation` self) _returnvalue) (`self.AttackRange`)))
    (`BlackboardComponent.SetValueAsBool` (`self.BB`) "IsChasing" true)
    (bind _asabp_enemy_zomb_new (cast `/Game/Blueprints/Enemies/ABP_EnemyZomb_New` (`SkeletalMeshComponent.GetAnimInstance` (`self.Mesh`))))
    (set `/Game/Blueprints/Enemies/ABP_EnemyZomb_New.IsRunning` true _asabp_enemy_zomb_new)
    (set `CharacterMovementComponent.MaxWalkSpeed` (* (`self.ChasingSpeed`) (- 1.0 (`self.SlowdownRate`))) (`self.CharacterMovement`))
    (`BlackboardComponent.SetValueAsBool` (`self.BB`) "HasTarget" true)
    (set `self.LastTimeSawPlayer` (`KismetSystemLibrary.GetGameTimeInSeconds`))))

(fn `Attack`
  (if (<= (`self.AttackTimer`) 0.0)
    (set `self.AttackTimer` (`self.AttackCooldown`))
    (bind _asabp_enemy_zomb_new (cast `/Game/Blueprints/Enemies/ABP_EnemyZomb_New` (`SkeletalMeshComponent.GetAnimInstance` (`self.Mesh`))))
    (set `/Game/Blueprints/Enemies/ABP_EnemyZomb_New.ShouldAttack` true _asabp_enemy_zomb_new)))

(fn `Die`
  (params (IsInflated :type Boolean))
  (bind _asbp_drone (cast `/Game/Blueprints/Drone/BP_Drone` (`GameplayStatics.GetPlayerPawn` 0)))
  (`/Game/Blueprints/Drone/BP_Drone.AddScore` _asbp_drone IsInflated)
  (if (not IsInflated)
    (`BrainComponent.StopLogic` (`AIController.BrainComponent` (`AIBlueprintHelperLibrary.GetAIController` null)) "")
    (bind _asabp_enemy_zomb_new (cast `/Game/Blueprints/Enemies/ABP_EnemyZomb_New` (`SkeletalMeshComponent.GetAnimInstance` (`self.Mesh`))))
    (set `/Game/Blueprints/Enemies/ABP_EnemyZomb_New.ShouldDie` true _asabp_enemy_zomb_new))
  (`|SpawnActorFromClass` "/Game/Blueprints/BP_EXPOrb.BP_EXPOrb_C" (`self.GetTransform`) "Undefined" "MultiplyWithRoot" null null)
  (bind _asgm_drone (cast `/Game/Core/GM_Drone` (`GameplayStatics.GetGameMode`)))
  (`/Game/Blueprints/Enemies/EnemyManager.ReportDeath` (`/Game/Core/GM_Drone.EnemyManager` _asgm_drone) self)
  (`self.K2_DestroyActor`))

(fn `Float`
  (bind _returnvalue (`self.K2_GetActorLocation` self))
  (bind _returnvalue_2 (+ _returnvalue (`KismetMathLibrary.MakeVector` 0.0 0.0 (`self.Portal_Height`))))
  (`BrainComponent.StopLogic` (`AIController.BrainComponent` (`AIBlueprintHelperLibrary.GetAIController` self)) "")
  (bind (_outhit _returnvalue_3) (`KismetSystemLibrary.LineTraceSingle` _returnvalue _returnvalue_2 "TraceTypeQuery1"))
  (bind _output_get (set `self.FloatingTarget` (select `bool` _returnvalue_3 :`false` _returnvalue_2 :`true` (`.Location` (`GameplayStatics.BreakHitResult` _outhit)))))
  (bind _returnvalue_4 (`|SpawnActorFromClass` "/Game/Blueprints/Portal/BP_Portal.BP_Portal_C" (`KismetMathLibrary.MakeTransform` _output_get) "AlwaysSpawn" "MultiplyWithRoot" null null))
  (set `self.Portal` _returnvalue_4)
  (bind _asabp_enemy_zomb_new (cast `/Game/Blueprints/Enemies/ABP_EnemyZomb_New` (`SkeletalMeshComponent.GetAnimInstance` (`self.Mesh`))))
  (set `/Game/Blueprints/Enemies/ABP_EnemyZomb_New.ShouldFloat` true _asabp_enemy_zomb_new)
  (`CharacterMovementComponent.DisableMovement` (`self.CharacterMovement`))
  (`PrimitiveComponent.SetCollisionEnabled` (`self.CapsuleComponent`) "NoCollision"))

(fn `HandleDamage`
  (params (BodyPartHit :type "PrimitiveComponent Object Reference") (Damage :type "Float (double-precision)")))

(fn `InflateBodyPart`
  (params (BodyPart :type "PrimitiveComponent Object Reference") (InflateValue :type "Float (double-precision)"))
  (locals (NewSlowdownRate :type "Float (double-precision)"))
  (bind _returnvalue (`KismetSystemLibrary.GetObjectName` BodyPart))
  (bind _bodypartinflation (`self.BodyPartInflation`))
  (bind _returnvalue_2 (`KismetMathLibrary.FMin` (+ (/ InflateValue 100.0) (`BlueprintMapLibrary.Map_Find` _bodypartinflation _returnvalue)) 1.0))
  (bind _output_get (set `local.NewSlowdownRate` (- (`self.SlowdownRate`) (`BlueprintMapLibrary.Map_Find` (`self.BodyPartInflation`) (`KismetSystemLibrary.GetObjectName` BodyPart)))))
  (`BlueprintMapLibrary.Map_Add` _bodypartinflation _returnvalue _returnvalue_2)
  (set `self.SlowdownRate` (+ _output_get (* _returnvalue_2 0.2)))
  (`self.SetChasePlayer`)
  (if (>= (`BlueprintMapLibrary.Map_Find` (`self.BodyPartInflation`) _returnvalue) 1.0)
    (if (not (`self.IsFloating`))
      (set `self.IsFloating` true)
      (`self.Float`))))

(fn `OnTakeDamage`
  (params (Damage :type "Float (double-precision)"))
  (`self.SetChasePlayer`)
  (if (not (`self.IsFloating`))
    (bind _output_get (set `self.Health` (- (`self.Health`) Damage)))
    (if (< _output_get 0.0)
      (`self.Die` false))))

(fn `SetChasePlayer`
  (set `self.AlwaysChasePlayer` true)
  (`BlackboardComponent.SetValueAsVector` (`self.BB`) "TargetPosition" (`self.K2_GetActorLocation` (`GameplayStatics.GetPlayerPawn` 0)))
  (`BlackboardComponent.SetValueAsObject` (`self.BB`) "TargetActor" (`GameplayStatics.GetPlayerPawn` 0))
  (`BlackboardComponent.SetValueAsBool` (`self.BB`) "IsChasing" true)
  (bind _asabp_enemy_zomb_new (cast `/Game/Blueprints/Enemies/ABP_EnemyZomb_New` (`SkeletalMeshComponent.GetAnimInstance` (`self.Mesh`))))
  (set `/Game/Blueprints/Enemies/ABP_EnemyZomb_New.IsRunning` true _asabp_enemy_zomb_new)
  (set `CharacterMovementComponent.MaxWalkSpeed` (* (`self.ChasingSpeed`) (- 1.0 (`self.SlowdownRate`))) (`self.CharacterMovement`))
  (`BlackboardComponent.SetValueAsBool` (`self.BB`) "HasTarget" true))

(fn `SetMovable`
  (params (IsMovable :type Boolean))
  (bind _bb (`self.BB`))
  (if IsMovable
    (`BlackboardComponent.SetValueAsBool` _bb "Movable" (`self.IsMovable`))
    (else
      (`BlackboardComponent.SetValueAsBool` _bb "Movable" false))))

(fn `SetPatrolDestination`
  (params (location :type "Vector Structure"))
  (`BlackboardComponent.SetValueAsVector` (`self.BB`) "TargetPosition" location)
  (`BlackboardComponent.SetValueAsBool` (`self.BB`) "HasTarget" true))

(fn `Shoot`
  (bind (_returnvalue_location _returnvalue_rotation _returnvalue_scale) (`KismetMathLibrary.BreakTransform` (`self.GetTransform` self)))
  (`|SpawnActorFromClass` (`self.Bullet`) (`KismetMathLibrary.MakeTransform` (+ _returnvalue_location (* (`self.GetActorForwardVector` self) 1.0)) (`KismetMathLibrary.FindLookAtRotation` _returnvalue_location (`self.K2_GetActorLocation` (`GameplayStatics.GetPlayerPawn` 0))) _returnvalue_scale) "AdjustIfPossibleButAlwaysSpawn" "MultiplyWithRoot" null null))

(fn `UserConstructionScript`
  (bind _returnvalue (`AIBlueprintHelperLibrary.GetAIController` self))
  (set `self.BB` (`AIBlueprintHelperLibrary.GetBlackboard` _returnvalue))
  (bind _asbp_enemy_aicontroller (cast `/Game/Blueprints/Enemies/BP_EnemyAIController` _returnvalue))
  (set `/Game/Blueprints/Enemies/BP_EnemyAIController.RoamRange` (`self.RoamRange`) _asbp_enemy_aicontroller)
  (`BlackboardComponent.SetValueAsBool` (`self.BB`) "Movable" (`self.IsMovable`))
  (`BlackboardComponent.SetValueAsBool` (`self.BB`) "WillAttack" (`self.WillAttack`))
  (if (`self.AlwaysChasePlayer`)
    (`BlackboardComponent.SetValueAsObject` (`self.BB`) "TargetActor" null)
    (`BlackboardComponent.SetValueAsBool` (`self.BB`) "HasTarget" true)))