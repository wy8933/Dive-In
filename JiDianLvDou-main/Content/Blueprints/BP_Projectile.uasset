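; BP_Projectile is a projectile actor that inflates the body part of an enemy it strikes.
; A Collider overlap with an actor tagged Enemy casts it to BP_EnemyBase and passes the hit component and an Inflation value to InflateBodyPart, then destroys the projectile.
; Blocking hits also destroy it, a 60-second timeout removes strays, and debug strings print the names of what it touches.
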(event `self.ReceiveBeginPlay`
  (`KismetSystemLibrary.Delay` 60.0)
  (`self.K2_DestroyActor`))

(event `self.ReceiveActorBeginOverlap`
  (params (OtherActor :type "Actor Object Reference")))

(event `self.Collider.OnComponentBeginOverlap`
  (params (OverlappedComponent :type "PrimitiveComponent Object Reference") (OtherActor :type "Actor Object Reference") (OtherComp :type "PrimitiveComponent Object Reference") (OtherBodyIndex :type Integer) (bFromSweep :type Boolean) (SweepResult :type "HitResult Structure (by ref)"))
  (if (`self.ActorHasTag` OtherActor "Enemy")
    (bind _asbp_enemy_base (cast `/Game/Blueprints/Enemies/BP_EnemyBase` OtherActor))
    (`KismetSystemLibrary.PrintString` (`KismetSystemLibrary.GetDisplayName` OtherComp))
    (`/Game/Blueprints/Enemies/BP_EnemyBase.InflateBodyPart` _asbp_enemy_base OtherComp (`self.Inflation`))
    (`self.K2_DestroyActor`)
    (else
      (`KismetSystemLibrary.PrintString` (`KismetSystemLibrary.GetDisplayName` OtherActor)))))

(event `self.Collider.OnComponentHit`
  (params (HitComponent :type "PrimitiveComponent Object Reference") (OtherActor :type "Actor Object Reference") (OtherComp :type "PrimitiveComponent Object Reference") (NormalImpulse :type "Vector Structure") (Hit :type "HitResult Structure (by ref)"))
  (`KismetSystemLibrary.PrintString` (`KismetSystemLibrary.GetDisplayName` OtherActor))
  (`self.K2_DestroyActor`))

(fn `UserConstructionScript`)