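; Behavior tree task that makes a BP_EnemyBase pawn attack the actor in the TargetActor blackboard key.
; On execute it stops AI movement, flags the enemy as attacking and reads the target.
; Each tick it smoothly yaws the enemy toward the target and calls Attack.
; It runs until aborted, then clears the flag and calls FinishExecute as failed.
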(event `self.ReceiveExecuteAI`
  (params (OwnerController :type "AIController Object Reference") (ControlledPawn :type "Pawn Object Reference"))
  (`Controller.StopMovement` OwnerController)
  (bind _asbp_enemy_base (cast `/Game/Blueprints/Enemies/BP_EnemyBase` ControlledPawn))
  (bind _output_get (set `self.Enemy` _asbp_enemy_base))
  (set `/Game/Blueprints/Enemies/BP_EnemyBase.IsAttacking` true _output_get)
  (bind _asactor (cast `Actor` (`BlackboardComponent.GetValueAsObject` (`AIBlueprintHelperLibrary.GetBlackboard` OwnerController) "TargetActor"))))

(event `self.ReceiveTickAI`
  (params (OwnerController :type "AIController Object Reference") (ControlledPawn :type "Pawn Object Reference") (DeltaSeconds :type "Float (single-precision)"))
  (bind (_returnvalue_location _returnvalue_rotation) (`KismetMathLibrary.BreakTransform` (`Actor.GetTransform` (`self.Enemy`))))
  (bind (_returnvalue_roll _returnvalue_pitch _returnvalue_yaw) (`KismetMathLibrary.BreakRotator` (`KismetMathLibrary.FindLookAtRotation` _returnvalue_location (`Actor.K2_GetActorLocation` (stale `self.ReceiveExecuteAI` _asactor)))))
  (`Actor.K2_SetActorRotation` (`self.Enemy`) (`KismetMathLibrary.RLerp` _returnvalue_rotation (`KismetMathLibrary.MakeRotator` 0.0 0.0 _returnvalue_yaw) (* DeltaSeconds 5.0) true) false)
  (`/Game/Blueprints/Enemies/BP_EnemyBase.Attack` (`self.Enemy`)))

(event `self.ReceiveAbortAI`
  (params (OwnerController :type "AIController Object Reference") (ControlledPawn :type "Pawn Object Reference"))
  (bind _asbp_enemy_base (cast `/Game/Blueprints/Enemies/BP_EnemyBase` ControlledPawn))
  (set `/Game/Blueprints/Enemies/BP_EnemyBase.IsAttacking` false _asbp_enemy_base)
  (`self.FinishExecute` false))