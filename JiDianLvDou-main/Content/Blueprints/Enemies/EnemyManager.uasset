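; Enemy manager that registers with GM_Drone, tracks all BP_EnemyBase actors and spawns patrols and chasers on timers, up to a population cap.
; Patrols spawn in randomly sized groups at tagged spawn points, using navigation path checks, and head to another point.
; Chasers spawn at random reachable points around the player, distance-checked against the manager's own location, then chase the player.
; ReportDeath removes enemies from the list and updates the count.
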(event `self.ReceiveBeginPlay`
  (bind _enemylist (`self.EnemyList`))
  (bind _outactors (`GameplayStatics.GetAllActorsOfClass` "/Game/Blueprints/Enemies/BP_EnemyBase.BP_EnemyBase_C"))
  (`KismetArrayLibrary.Array_Append` _enemylist _outactors)
  (set `self.CurrentEnemyNumber` (`KismetArrayLibrary.Array_Length` _enemylist))
  (bind _asgm_drone (cast `/Game/Core/GM_Drone` (`GameplayStatics.GetGameMode`)))
  (set `/Game/Core/GM_Drone.EnemyManager` self _asgm_drone)
  (bind _outactors_2 (`GameplayStatics.GetAllActorsWithTag` "EnemySpawnPoint"))
  (for _array_element _outactors_2
    (`KismetArrayLibrary.Array_Add` (`self.SpawnPoints`) (`self.GetTransform` _array_element))))

(event `self.ReceiveTick`
  (params (DeltaSeconds :type "Float (single-precision)"))
  (bind _returnvalue (+ DeltaSeconds (`self.ChaserTimer`)))
  (bind _returnvalue_2 (+ DeltaSeconds (`self.PatrolTimer`)))
  (if (> _returnvalue_2 (`self.PatrolSpawnInterval`))
    (`self.SpawnPatrol`)
    (set `self.PatrolTimer` 0.0)
    (else
      (set `self.PatrolTimer` _returnvalue_2)))
  (if (> _returnvalue (`self.ChaserSpawnInterval`))
    (`self.SpawnChaser`)
    (set `self.ChaserTimer` 0.0)
    (else
      (set `self.ChaserTimer` _returnvalue))))

(fn `ReportDeath`
  (params (Enemy :type "/Game/Blueprints/Enemies/BP_EnemyBase Object Reference"))
  (`KismetArrayLibrary.Array_RemoveItem` (`self.EnemyList`) Enemy)
  (set `self.CurrentEnemyNumber` (`KismetArrayLibrary.Array_Length` (`self.EnemyList`))))

(fn `SpawnChaser`
  (locals (ID :type Integer :default -1) (SpawnCamp :type "Vector Structure" :default (0.0 0.0 0.0)) (DestCamp :type "Vector Structure" :default (0.0 0.0 0.0)) (Unreachable :type Boolean :default false) (Position :type "Vector Structure" :default (0.0 0.0 0.0)) (LoopCounter :type Integer))
  (bind _returnvalue_location (`KismetMathLibrary.BreakTransform` (`self.GetTransform` (`GameplayStatics.GetPlayerPawn` 0))))
  (bind (_randomlocation _returnvalue) (`NavigationSystemV1.K2_GetRandomReachablePointInRadius` _returnvalue_location (`self.MaxSpawnRadius`) null null))
  (if (`self.WillSpawnChaser`)
    (if (< (`self.CurrentEnemyNumber`) (`self.MaximumEnemyNumber`))
      (set `local.LoopCounter` 0)
      (while (and (or (== (`KismetMathLibrary.VSize` (`local.Position`)) 0.0) (< (`KismetMathLibrary.Vector_Distance` (`local.Position`) (`self.K2_GetActorLocation` self)) (`self.MinSpawnRadius`))) (<= (`local.LoopCounter`) 100))
        (set `local.LoopCounter` (+ (`local.LoopCounter`) 1))
        (if _returnvalue
          (set `local.Position` _randomlocation)))
      (bind _returnvalue_2 (`|SpawnActorFromClass` "/Game/Blueprints/Enemies/BP_EnemyBase.BP_EnemyBase_C" (`KismetMathLibrary.MakeTransform` (`local.Position`)) "AdjustIfPossibleButAlwaysSpawn" "MultiplyWithRoot" null null))
      (set `/Game/Blueprints/Enemies/BP_EnemyBase.Manager` self _returnvalue_2)
      (bind _returnvalue_3 (`KismetArrayLibrary.Array_Add` (`self.EnemyList`) _returnvalue_2))
      (set `self.CurrentEnemyNumber` _returnvalue_3)
      (`/Game/Blueprints/Enemies/BP_EnemyBase.SetChasePlayer` _returnvalue_2))))

(fn `SpawnPatrol`
  (locals (ID :type Integer :default -1) (SpawnCamp :type "Vector Structure" :default (0.0 0.0 0.0)) (DestCamp :type "Vector Structure" :default (0.0 0.0 0.0)) (Unreachable :type Boolean :default true))
  (bind _groupsizevariant (`self.GroupSizeVariant`))
  (bind (_outitem _outindex) (`KismetArrayLibrary.Array_Random` (`self.SpawnPoints`)))
  (bind (_outitem_2 _outindex_2) (`KismetArrayLibrary.Array_Random` (`self.SpawnPoints`)))
  (if (`self.WillSpawnPatrol`)
    (set `local.DestCamp` (.location _outitem_2))
    (while (or (== _outindex_2 (`local.ID`)) (`local.Unreachable`))
      (set `local.SpawnCamp` (.location _outitem))
      (set `local.ID` _outindex)
      (bind _returnvalue (`NavigationSystemV1.FindPathToLocationSynchronously` (`local.SpawnCamp`) (`local.DestCamp`) null null))
      (set `local.Unreachable` (`NavigationPath.IsPartial` _returnvalue)))
    (for _ (range 1 (+ (`KismetMathLibrary.Min` (+ (`self.PatrolGroupSize`) (`KismetMathLibrary.RandomIntegerInRange` (* _groupsizevariant -1) _groupsizevariant)) (- (`self.MaximumEnemyNumber`) (`self.CurrentEnemyNumber`))) 1))
      (bind _returnvalue_2 (`|SpawnActorFromClass` "/Game/Blueprints/Enemies/BP_EnemyBase.BP_EnemyBase_C" (`KismetMathLibrary.MakeTransform` (`NavigationSystemV1.K2_GetRandomReachablePointInRadius` (`local.SpawnCamp`) 5.0 null null)) "AdjustIfPossibleButAlwaysSpawn" "MultiplyWithRoot" null null))
      (set `/Game/Blueprints/Enemies/BP_EnemyBase.Manager` self _returnvalue_2)
      (bind _returnvalue_3 (`KismetArrayLibrary.Array_Add` (`self.EnemyList`) _returnvalue_2))
      (set `self.CurrentEnemyNumber` _returnvalue_3)
      (`/Game/Blueprints/Enemies/BP_EnemyBase.SetPatrolDestination` _returnvalue_2 (`NavigationSystemV1.K2_GetRandomReachablePointInRadius` (`local.DestCamp`) 50.0 null null)))))

(fn `UserConstructionScript`)