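; BP_EnemyAIController is the AI controller for BP_EnemyBase enemies, running the BT_EnemyBase behavior tree on possession.
; It hands the Blackboard to the possessed enemy and seeds its movement and attack flags from that enemy's settings.
; Enemies set to always chase the player start with player pawn 0 as their target.
; A RoamRange assignment is left disconnected and never runs.
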(event `self.ReceivePossess`
  (params (PossessedPawn :type "Pawn Object Reference"))
  (bind _returnvalue (`AIBlueprintHelperLibrary.GetBlackboard` null))
  (`self.RunBehaviorTree` "/Game/Blueprints/Enemies/BT_EnemyBase.BT_EnemyBase")
  (bind _asbp_enemy_base (cast `/Game/Blueprints/Enemies/BP_EnemyBase` PossessedPawn))
  (set `/Game/Blueprints/Enemies/BP_EnemyBase.BB` _returnvalue _asbp_enemy_base)
  (`BlackboardComponent.SetValueAsBool` _returnvalue "Movable" (`/Game/Blueprints/Enemies/BP_EnemyBase.IsMovable` _asbp_enemy_base))
  (`BlackboardComponent.SetValueAsBool` _returnvalue "WillAttack" (`/Game/Blueprints/Enemies/BP_EnemyBase.WillAttack` _asbp_enemy_base))
  (if (`/Game/Blueprints/Enemies/BP_EnemyBase.AlwaysChasePlayer` _asbp_enemy_base)
    (`BlackboardComponent.SetValueAsObject` _returnvalue "TargetActor" (`GameplayStatics.GetPlayerPawn` 0))
    (`BlackboardComponent.SetValueAsBool` _returnvalue "HasTarget" true)))

(fn `UserConstructionScript`)