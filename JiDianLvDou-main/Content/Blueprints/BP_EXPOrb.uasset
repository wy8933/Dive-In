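; BP_EXPOrb is an experience pickup that homes in on a BP_Drone and grants it EXP.
; Overlapping the CatchRadius component stores the drone as the target and enables pursuit, which stops when a drone leaves the radius.
; Each Tick moves the orb straight toward the target at a constant Speed without sweeping.
; Once closer than Distance, it calls AddEXP on the drone and destroys itself.
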(event `self.ReceiveTick`
  (params (DeltaSeconds :type "Float (single-precision)"))
  (bind _returnvalue (- (`self.K2_GetActorLocation` (`self.TargetActor`)) (`self.K2_GetActorLocation`)))
  (if (`self.IsInRadius`)
    (if (< (`KismetMathLibrary.VSize` _returnvalue) (`self.Distance`))
      (bind _asbp_drone (cast `/Game/Blueprints/Drone/BP_Drone` (`self.TargetActor`)))
      (`/Game/Blueprints/Drone/BP_Drone.AddEXP` _asbp_drone (`self.EXPAmount`))
      (`self.K2_DestroyActor`)
      (else
        (`self.K2_SetActorLocation` (+ (* (`KismetMathLibrary.Normal` _returnvalue) (* (`self.Speed`) DeltaSeconds)) (`self.K2_GetActorLocation`)))))))

(event `self.CatchRadius.OnComponentBeginOverlap`
  (params (OverlappedComponent :type "PrimitiveComponent Object Reference") (OtherActor :type "Actor Object Reference") (OtherComp :type "PrimitiveComponent Object Reference") (OtherBodyIndex :type Integer) (bFromSweep :type Boolean) (SweepResult :type "HitResult Structure (by ref)"))
  (bind _asbp_drone (cast `/Game/Blueprints/Drone/BP_Drone` OtherActor))
  (set `self.TargetActor` _asbp_drone)
  (set `self.IsInRadius` true))

(event `self.CatchRadius.OnComponentEndOverlap`
  (params (OverlappedComponent :type "PrimitiveComponent Object Reference") (OtherActor :type "Actor Object Reference") (OtherComp :type "PrimitiveComponent Object Reference") (OtherBodyIndex :type Integer))
  (cast `/Game/Blueprints/Drone/BP_Drone` OtherActor)
  (set `self.IsInRadius` false))

(fn `UserConstructionScript`)