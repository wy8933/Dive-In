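; Play-area boundary volume that gives the player's BP_Drone a short grace period to return after leaving, or the game is lost.
; Exiting the Trigger starts a timer and shows WBP_OutOfBound, which Tick updates with the remaining time; re-entering cancels both.
; On timeout it shows WBP_Lose with the current enemy count from GM_Drone's EnemyManager, switches to UI-only input and pauses the game.
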(event `self.ReceiveTick`
  (params (DeltaSeconds :type "Float (single-precision)"))
  (if (not (`self.PlayerInside`))
    (`/Game/Blueprints/WBP/WBP_OutOfBound.SetTimer` (`self.OutOfBoundWidget`) (`KismetSystemLibrary.K2_GetTimerRemainingTimeHandle` (`self.LoseTimerHandle`)))))

(event `self.Trigger.OnComponentEndOverlap`
  (params (OverlappedComponent :type "PrimitiveComponent Object Reference") (OtherActor :type "Actor Object Reference") (OtherComp :type "PrimitiveComponent Object Reference") (OtherBodyIndex :type Integer))
  (if (`self.PlayerInside`)
    (bind _asbp_drone (cast `/Game/Blueprints/Drone/BP_Drone` OtherActor))
    (set `self.Drone` _asbp_drone)
    (set `self.PlayerInside` false)
    (`KismetSystemLibrary.K2_ClearAndInvalidateTimerHandle` (`self.LoseTimerHandle`))
    (bind _returnvalue (`KismetSystemLibrary.K2_SetTimerDelegate` (delegate `TimeOut`) 5.0))
    (set `self.LoseTimerHandle` _returnvalue)
    (bind _returnvalue_2 (`|CreateWidget` "/Game/Blueprints/WBP/WBP_OutOfBound.WBP_OutOfBound_C" (`GameplayStatics.GetPlayerController` 0)))
    (bind _output_get (set `self.OutOfBoundWidget` _returnvalue_2))
    (`UserWidget.AddToViewport` _output_get 0)))

(event `self.Trigger.OnComponentBeginOverlap`
  (params (OverlappedComponent :type "PrimitiveComponent Object Reference") (OtherActor :type "Actor Object Reference") (OtherComp :type "PrimitiveComponent Object Reference") (OtherBodyIndex :type Integer) (bFromSweep :type Boolean) (SweepResult :type "HitResult Structure (by ref)"))
  (if (not (`self.PlayerInside`))
    (cast `/Game/Blueprints/Drone/BP_Drone` OtherActor)
    (set `self.PlayerInside` true)
    (`KismetSystemLibrary.K2_ClearAndInvalidateTimerHandle` (`self.LoseTimerHandle`))
    (`Widget.RemoveFromParent` (`self.OutOfBoundWidget`))))

(event `TimeOut`
  (bind _returnvalue (`GameplayStatics.GetPlayerController` 0))
  (`Widget.RemoveFromParent` (`self.OutOfBoundWidget`))
  (bind _returnvalue_2 (`|CreateWidget` "/Game/Blueprints/WBP/WBP_Lose.WBP_Lose_C" (`GameplayStatics.GetPlayerController` 0)))
  (bind _asgm_drone (cast `/Game/Core/GM_Drone` (`GameplayStatics.GetGameMode`)))
  (`/Game/Blueprints/WBP/WBP_Lose.Init` _returnvalue_2 (`KismetMathLibrary.Conv_IntToInt64` (`/Game/Blueprints/Enemies/EnemyManager.CurrentEnemyNumber` (`/Game/Core/GM_Drone.EnemyManager` _asgm_drone))))
  (`UserWidget.AddToViewport` _returnvalue_2 0)
  (`WidgetBlueprintLibrary.SetInputMode_UIOnlyEx` _returnvalue null)
  (set `PlayerController.bShowMouseCursor` true _returnvalue)
  (`GameplayStatics.SetGamePaused` true))

(fn `UserConstructionScript`)